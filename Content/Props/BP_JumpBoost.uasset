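; Jump boost pickup that temporarily changes the jump velocity of a BP_ThirdPersonCharacter overlapping its sphere.
; On overlap it plays two 2D sounds, hides its mesh and sets JumpZVelocity to the boost amount.
; After a delay it restores the stored OriginalJumpZ value, which is not read from the character here, and shows the mesh again.
; The sphere's collision stays active while the mesh is hidden.
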(event OnComponentBeginOverlap(Sphere)
  (params (OverlappedComponent :type Primitive%20Component%20Object%20Reference) (OtherActor :type Actor%20Object%20Reference) (OtherComp :type Primitive%20Component%20Object%20Reference) (OtherBodyIndex :type Integer) (bFromSweep :type Boolean) (SweepResult :type Hit%20Result%20Structure%20%28by%20ref%29))
  (bind _asbp_third_person_character (Utilities|Casting|CastToBP_ThirdPersonCharacter OtherActor))
  (Audio|PlaySound2D "/Game/Sound/S_PowerUp.S_PowerUp" 1.0 1.0 0.0 0 0)
  (Audio|PlaySound2D "/Game/Sound/S_Lick.S_Lick" 1.0 1.0 26.0 0 0)
  (Rendering|SetVisibility (Variables|Default|Getfbx) false false)
  (Variables|/Script/Engine.CharacterMovementComponent|SetJumpZVelocity (Variables|/Script/Engine.Character|GetCharacterMovement _asbp_third_person_character) (Variables|Default|GetJumpBoostAmount))
  (Utilities|FlowControl|Delay (Variables|Default|GetBoostDuration))
  (Variables|/Script/Engine.CharacterMovementComponent|SetJumpZVelocity (Variables|/Script/Engine.Character|GetCharacterMovement _asbp_third_person_character) (Variables|Default|GetOriginalJumpZ))
  (Rendering|SetVisibility (Variables|Default|Getfbx) true false))

(event EventBeginPlay)

(event Collision|EventActorBeginOverlap
  (params (OtherActor :type Actor%20Object%20Reference)))

(event EventTick
  (params (DeltaSeconds :type Float%20%28single-precision%29)))

(fn ConstructionScript)