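; BP_Door2 is a door prop that swings open when the player approaches and closes when they leave.
; A box trigger's begin overlap checks for the player's third-person character and calls OpenDoor, while end overlap calls CloseDoor.
; A DoorAnimation timeline drives a rotation lerp that turns the door to 110 degrees of yaw, and closing plays it in reverse.
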(event OnComponentBeginOverlap(Box)
  (params (OverlappedComponent :type Primitive%20Component%20Object%20Reference) (OtherActor :type Actor%20Object%20Reference) (OtherComp :type Primitive%20Component%20Object%20Reference) (OtherBodyIndex :type Integer) (bFromSweep :type Boolean) (SweepResult :type Hit%20Result%20Structure%20%28by%20ref%29))
  (Utilities|Casting|CastToBP_ThirdPersonCharacter OtherActor)
  (if (== OtherActor (Game|GetPlayerCharacter 0))
    (CallFunction|OpenDoor)))

(event OnComponentEndOverlap(Box)
  (params (OverlappedComponent :type Primitive%20Component%20Object%20Reference) (OtherActor :type Actor%20Object%20Reference) (OtherComp :type Primitive%20Component%20Object%20Reference) (OtherBodyIndex :type Integer))
  (if (== OtherActor (Game|GetPlayerCharacter 0))
    (CallFunction|CloseDoor)))

(event Custom|Open%20Door
  (bind _door_alpha (Timeline|DoorAnimation Play)
    (:Update
      (Transformation|SetRelativeRotation (Variables|Default|GetDoor) (Math|Rotator|Lerp(Rotator) "0, 0, 0" "0.000000,110.000000,0.000000" _door_alpha true) false false))))

(event Custom|Close%20Door
  (bind _door_alpha (Timeline|DoorAnimation Reverse)
    (:Update
      (Transformation|SetRelativeRotation (Variables|Default|GetDoor) (Math|Rotator|Lerp(Rotator) "0, 0, 0" "0.000000,110.000000,0.000000" _door_alpha true) false false))))

(fn ConstructionScript)