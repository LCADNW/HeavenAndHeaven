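; BP_JumpBoost2 is a jump boost pickup that temporarily changes the jump velocity of a third-person character that overlaps its sphere.
; On overlap it hides its mesh, starts an attached power-up sound loop and sets the character's JumpZVelocity to the boost amount.
; After a delay it sets JumpZVelocity to a stored original value, shows the mesh again and stops the audio.
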(event OnComponentBeginOverlap(Sphere)
  (params (OverlappedComponent :type Primitive%20Component%20Object%20Reference) (OtherActor :type Actor%20Object%20Reference) (OtherComp :type Primitive%20Component%20Object%20Reference) (OtherBodyIndex :type Integer) (bFromSweep :type Boolean) (SweepResult :type Hit%20Result%20Structure%20%28by%20ref%29))
  (bind _asbp_third_person_character (Utilities|Casting|CastToBP_ThirdPersonCharacter OtherActor))
  (bind _returnvalue (Audio|SpawnSoundAttached "/Game/Sound/S_PowerUpLoop.S_PowerUpLoop" (Variables|Default|Getfbx) "None" "0, 0, 0" "0, 0, 0" "KeepRelativeOffset" false 1.0 1.0 0.0 0 0))
  (Variables|Default|SetPowerUpAudio _returnvalue)
  (Rendering|SetVisibility (Variables|Default|Getfbx) false false)
  (Variables|/Script/Engine.CharacterMovementComponent|SetJumpZVelocity (Variables|/Script/Engine.Character|GetCharacterMovement _asbp_third_person_character) (Variables|Default|GetJumpBoostAmount))
  (Utilities|FlowControl|Delay (Variables|Default|GetBoostDuration))
  (Variables|/Script/Engine.CharacterMovementComponent|SetJumpZVelocity (Variables|/Script/Engine.Character|GetCharacterMovement _asbp_third_person_character) (Variables|Default|GetOriginalJumpZ))
  (Rendering|SetVisibility (Variables|Default|Getfbx) true false)
  (Audio|Components|Audio|FadeOut (Variables|Default|GetPowerUpAudio) 0.0 0.0 "Linear" :!class /Script/Engine.AudioComponent))

(fn ConstructionScript)