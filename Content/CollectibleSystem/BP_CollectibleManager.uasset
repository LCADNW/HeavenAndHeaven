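; BP_CollectibleManager keeps a running total for each collectible type, such as Scrap and Orb.
; On BeginPlay it finds every BP_Collectibles actor in the level and binds to its OnCollected event.
; Each pickup adds its value to the type's entry in CollectibleDict, then broadcasts the map through OnTotalUpdated.
; ResetTotal clears the map and broadcasts the same update.
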(event Custom|OnCollected_Event
  (params (Type :type E_CollectibleType%20Enum :default "NewEnumerator0") (Value :type Integer))
  (CallFunction|AddCollectible Type Value))

(event EventBeginPlay
  (bind _outactors (Actor|GetAllActorsOfClass "/Game/CollectibleSystem/BP_Collectibles.BP_Collectibles_C"))
  (EventDispatchers|BindEventtoOnCollected _outactors (delegate Custom|OnCollected_Event)))

(fn ConstructionScript)

(fn AddCollectible
  (params (CollectibleType :type E_CollectibleType%20Enum :default "NewEnumerator0") (Collectible%20Value :type Integer))
  (Utilities|Map|Add (Variables|Default|GetCollectibleDict) CollectibleType (+ Collectible%20Value (.Value (Utilities|Map|Find (Variables|Default|GetCollectibleDict) (Variables|Default|GetCollectibleType)))))
  (Default|CallOnTotalUpdated (Variables|Default|GetCollectibleDict)))

(fn ResetTotal
  (bind _collectibledict (Variables|Default|GetCollectibleDict))
  (Utilities|Map|Clear _collectibledict)
  (Default|CallOnTotalUpdated _collectibledict))