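; BP_PlayerState is the player state for the collectible system, keeping a running total for each collectible type.
; On BeginPlay it binds to the OnCollected event of BP_Collectibles actors found in the level, so later spawns are not bound.
; Each pickup adds its value to that type's entry in the CollectibleDict map.
; AddCollectible and ResetCollectible, which clears the map, both broadcast OnTotalUpdated with the map.
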(event Custom|OnCollected_Event
  (params (Type :type E_CollectibleType%20Enum :default "NewEnumerator0") (Value :type Integer))
  (CallFunction|AddCollectible Type Value))

(event EventBeginPlay
  (bind _outactors (Actor|GetAllActorsOfClass "/Game/CollectibleSystem/BP_Collectibles.BP_Collectibles_C"))
  (EventDispatchers|BindEventtoOnCollected _outactors (delegate Custom|OnCollected_Event)))

(fn ConstructionScript)

(fn AddCollectible
  (params (ColType :type E_CollectibleType%20Enum :default "NewEnumerator0") (ColValue :type Integer))
  (Utilities|Map|Add (Variables|Default|GetCollectibleDict) ColType (+ ColValue (.Value (Utilities|Map|Find (Variables|Default|GetCollectibleDict) ColType))))
  (Default|CallOnTotalUpdated (Variables|Default|GetCollectibleDict)))

(fn ResetCollectible
  (bind _collectibledict (Variables|Default|GetCollectibleDict))
  (Utilities|Map|Clear _collectibledict)
  (Default|CallOnTotalUpdated _collectibledict))